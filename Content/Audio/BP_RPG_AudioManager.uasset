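; Audio manager actor that starts the game's music on play and exposes volume controls for music and sound effects.
; Volume setters apply sound class overrides on RPG_SoundMix for the RPG_Music and RPG_SFX classes with no fade.
; Setting music volume to near zero flags the music as stopped, and a later non-zero volume replays the track from the start as a 2D sound.
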(event EventBeginPlay
  (CallFunction|StartMusic))

(event Collision|EventActorBeginOverlap
  (params (OtherActor :type Actor%20Object%20Reference)))

(event EventTick
  (params (DeltaSeconds :type Float%20%28single-precision%29)))

(fn ConstructionScript)

(fn SetSFXVolume
  (params (Value :type Float%20%28single-precision%29))
  (Audio|SetSoundMixClassOverride "/Game/Audio/RPG_SoundMix.RPG_SoundMix" "/Game/Audio/RPG_SFX.RPG_SFX" Value 1.0 0.0 true))

(fn SetMusicVolume
  (params (Value :type Float%20%28single-precision%29))
  (Audio|SetSoundMixClassOverride "/Game/Audio/RPG_SoundMix.RPG_SoundMix" "/Game/Audio/RPG_Music.RPG_Music" Value 1.0 0.0 true)
  (if (Math|Float|NearlyEqual(Float) Value 0.0 1e-06)
    (Variables|Default|SetMusicStopped true)
    (elif (Variables|Default|GetMusicStopped)
      (CallFunction|StartMusic))))

(fn StartMusic
  (Audio|PlaySound2D "/Game/Assets/Music/mm_music.mm_music" 1.0 1.0 0.0 0 0)
  (Variables|Default|SetMusicStopped false))