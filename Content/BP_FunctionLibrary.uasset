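; BP_FunctionLibrary is a function library of shared shortcuts to RPG game systems.
; RPGShowMessage casts player 0's controller and HUD to their RPG classes, then forwards a timed message to the GameHUD.
; GetRPGEventManager returns the EventManager held by the RPG game state.
; Both helpers stop without effect if a cast fails.
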(fn RPGShowMessage
  (params (Context :type Actor%20Object%20Reference) (Message :type String) (Duration :type Float%20%28single-precision%29))
  (bind _asrpgplayer_controller (Utilities|Casting|CastToRPGPlayerController (Game|GetPlayerController Context)))
  (bind _asrpg_hud (Utilities|Casting|CastToRPG_HUD (HUD|GetHUD _asrpgplayer_controller)))
  (Class|RPGGameHUD|ShowMessage (Variables|/Script/RPG.RPG_HUD|GetGameHUD _asrpg_hud) Message Duration))

(fn GetRPGEventManager
  (bind _asrpg_game_state_base (Utilities|Casting|CastToRPG_GameStateBase (Game|GetGameState (LocalVariables|Get__WorldContext))))
  (return (Variables|/Script/RPG.RPG_GameStateBase|GetEventManager _asrpg_game_state_base)))