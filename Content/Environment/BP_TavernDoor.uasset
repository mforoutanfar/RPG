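; Interactable tavern door that stays locked while hostiles remain in the area.
; On BeginPlay it subscribes to the RPG event manager's hostile-state change and sets its locked flag from the inverse of the clear state.
; Interacting while locked shows a message and plays a locked sound; otherwise it fires the "Tavern" story event through the event manager.
; It reports the door interactable type in either state.
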(event Custom|HostileStateChanged_Event_0
  (params (Clear :type Boolean))
  (Variables|Default|SetLocked (not Clear)))

(event EventBeginPlay
  (bind _eventmanager (CallFunction|GetRPGEventManager))
  (EventDispatchers|AssignHostileStateChanged _eventmanager (delegate Custom|HostileStateChanged_Event_0)))

(event Collision|EventActorBeginOverlap
  (params (OtherActor :type Actor%20Object%20Reference)))

(event EventTick
  (params (DeltaSeconds :type Float%20%28single-precision%29)))

(event EventOnInteracted
  (params (Successful :type Boolean))
  (if (Variables|Default|GetLocked)
    (CallFunction|RPGShowMessage self "Tavern closed until all hostiles are eliminated. " 5.0)
    (Audio|PlaySoundatLocation "/Game/Assets/Sounds/locked0.locked0" (Transformation|GetActorLocation) "0, 0, 0" 1.0 1.0 0.0 0 0 0)
    (else
      (bind _eventmanager (CallFunction|GetRPGEventManager))
      (Default|CallStoryEventTriggered _eventmanager "Tavern"))))

(fn ConstructionScript)

(fn GetInteractableType
  (if (Variables|Default|GetLocked)
    (return "LOCKED_DOOR")
    (else
      (return "DOOR"))))