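; BP_Lift is a lift actor that moves between two positions when any of its linked RPG buttons is pressed.
; On BeginPlay it binds each button's press event and records its start location.
; A press sets the other buttons pressed, waits briefly, then plays a sound while a timeline moves the actor along DeltaPos, forward or reversed.
; On finish it stops the sound, notifies all buttons and flips CurrentPos.
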(event Custom|RPGButtonPressed_Event_0
  (params (Button :type Actor%20Object%20Reference))
  (for _array_element (Variables|Default|GetButtons)
    (if (!= Button _array_element)
      (Default|OnRPGButtonPressed _array_element)
      (Class|RPGButton|SetIsPressed _array_element true)))
  (Utilities|FlowControl|Delay 1.0)
  (Audio|Components|Audio|Play (Variables|Default|Getlift_sfx) 0.0)
  (if (== (Variables|Default|GetCurrentPos) 0)
    (bind _newtrack_0 (Timeline|Timeline_0 PlayFromStart)
      (:Update
        (Transformation|SetActorLocation (+ (* (Variables|Default|GetDeltaPos) _newtrack_0) (Variables|Default|GetInitPos)) false false))
      (:Finished
        (Audio|Components|Audio|Stop (Variables|Default|Getlift_sfx))
        (for _array_element_2 (Variables|Default|GetButtons)
          (Default|FunctionFinished _array_element_2))
        (if (== (Variables|Default|GetCurrentPos) 0)
          (Variables|Default|SetCurrentPos 1)
          (else
            (Variables|Default|SetCurrentPos 0)))))
    (else
      (Timeline|Timeline_0 ReverseFromEnd))))

(event EventBeginPlay
  (for _array_element (Variables|Default|GetButtons)
    (EventDispatchers|AssignRPGButtonPressed _array_element (delegate Custom|RPGButtonPressed_Event_0))
    (Variables|Default|SetInitPos (Transformation|GetActorLocation))))

(event Collision|EventActorBeginOverlap
  (params (OtherActor :type Actor%20Object%20Reference)))

(event EventTick
  (params (DeltaSeconds :type Float%20%28single-precision%29)))

(fn ConstructionScript)