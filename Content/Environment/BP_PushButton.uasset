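; BP_PushButton is a push button actor that animates and clicks when its RPG button press event fires.
; BeginPlay stores the Mover's position, binds the press event and creates a dynamic material.
; A press plays two delayed clicks while a timeline shifts the Mover along local X and drives its ButtonColor parameter.
; FunctionFinished calls OnRPGButtonFunctionFinished and reverses the timeline, restoring the button's position and color.
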(event Custom|OnRPGButtonPressed
  (params (Button :type Actor%20Object%20Reference))
  (bind _buttoninitpos (Variables|Default|GetButtonInitPos))
  (Utilities|FlowControl|Sequence
    (:then_0
      (Audio|PlaySound2D "/Game/Assets/Sounds/click0.click0" 1.0 1.0 0.0 0 0)
      (Utilities|FlowControl|Delay 0.3)
      (Audio|PlaySound2D "/Game/Assets/Sounds/click1.click1" 1.0 1.0 0.0 0 0))
    (:then_1
      (bind (_direction _buttondisplacement _buttoncolor) (Timeline|Timeline_0 PlayFromStart)
        (:Update
          (Transformation|SetRelativeLocation (Variables|Default|GetMover) (Math|Vector|MakeVector (+ _buttondisplacement (.x _buttoninitpos)) (.y _buttoninitpos) (.z _buttoninitpos)) false false)
          (Rendering|Material|SetVectorParameterValue (Variables|Default|GetDynMat) "ButtonColor" _buttoncolor :!class /Script/Engine.MaterialInstanceDynamic))))))

(event Custom|FunctionFinished
  (bind _buttoninitpos (Variables|Default|GetButtonInitPos))
  (Class|RPGButton|OnRPGButtonFunctionFinished)
  (bind (_direction _buttondisplacement _buttoncolor) (Timeline|Timeline_0 ReverseFromEnd)
    (:Update
      (Transformation|SetRelativeLocation (Variables|Default|GetMover) (Math|Vector|MakeVector (+ _buttondisplacement (.x _buttoninitpos)) (.y _buttoninitpos) (.z _buttoninitpos)) false false)
      (Rendering|Material|SetVectorParameterValue (Variables|Default|GetDynMat) "ButtonColor" _buttoncolor :!class /Script/Engine.MaterialInstanceDynamic))))

(event EventBeginPlay
  (Variables|Default|SetButtonInitPos (Variables|/Script/Engine.SceneComponent|GetRelativeLocation (Variables|Default|GetMover)))
  (EventDispatchers|AssignRPGButtonPressed (delegate Custom|OnRPGButtonPressed))
  (bind _returnvalue (Rendering|Material|CreateDynamicMaterialInstance (Variables|Default|GetMover) 0 "/Game/Environment/ButtonMaterial.ButtonMaterial" "None" :!class /Script/Engine.PrimitiveComponent))
  (Variables|Default|SetDynMat _returnvalue))

(event Collision|EventActorBeginOverlap
  (params (OtherActor :type Actor%20Object%20Reference)))

(event EventTick
  (params (DeltaSeconds :type Float%20%28single-precision%29)))

(fn ConstructionScript)