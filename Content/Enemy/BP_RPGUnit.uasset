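; BP_RPGUnit is an enemy unit Blueprint that gives audio and visual feedback when the unit becomes alerted.
; The alert indicator, AlertNode, is hidden on BeginPlay.
; SetIsAlert stores the state and, when true, plays a random alert sound, shows AlertNode and scales it uniformly through a timeline.
; The indicator hides again when the timeline finishes, while setting the state to false only updates the flag.
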(event Custom|SetIsAlert
  (params (Alert :type Boolean))
  (bind _alertnode (Variables|Default|GetAlertNode))
  (bind _output_get (Variables|Default|SetIsAlert Alert))
  (if _output_get
    (Class|RPGRandomAudioComponent|PlayRandom (Variables|Default|GetAudioComponent) (Variables|Default|GetAlertSound))
    (Rendering|SetVisibility (Variables|Default|GetAlertNode) true true)
    (bind _newtrack_0 (Timeline|Timeline_0 PlayFromStart)
      (:Update
        (Transformation|SetWorldScale3D _alertnode (Math|Vector|MakeVector _newtrack_0 _newtrack_0 _newtrack_0)))
      (:Finished
        (Rendering|SetVisibility _alertnode false true)))))

(event EventBeginPlay
  (Rendering|SetVisibility (Variables|Default|GetAlertNode) false true))

(event Collision|EventActorBeginOverlap
  (params (OtherActor :type Actor%20Object%20Reference)))

(event EventTick
  (params (DeltaSeconds :type Float%20%28single-precision%29)))

(fn ConstructionScript)