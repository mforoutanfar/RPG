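; BP_Gong is an interactable gong that spawns a new enemy wave when used.
; It tracks whether hostiles are cleared through the RPG event manager's HostileStateChanged event, and shows a refusal message if interacted with while they remain.
; A successful interaction calls the GameState's SpawnManager, shows a message, plays the gong sound and runs a timeline that offsets the Sphere along X from its initial position.
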(event Custom|HostileStateChanged_Event_0
  (params (Clear :type Boolean))
  (Variables|Default|SetClear Clear))

(event EventBeginPlay
  (bind _eventmanager (CallFunction|GetRPGEventManager))
  (EventDispatchers|AssignHostileStateChanged _eventmanager (delegate Custom|HostileStateChanged_Event_0))
  (Variables|Default|SetInitPos (Variables|/Script/Engine.SceneComponent|GetRelativeLocation (Variables|Default|GetSphere))))

(event Collision|EventActorBeginOverlap
  (params (OtherActor :type Actor%20Object%20Reference)))

(event EventTick
  (params (DeltaSeconds :type Float%20%28single-precision%29)))

(event EventOnInteracted
  (params (Successful :type Boolean))
  (bind _initpos (Variables|Default|GetInitPos))
  (if (Variables|Default|GetClear)
    (bind _asrpg_game_state_base (Utilities|Casting|CastToRPG_GameStateBase (Game|GetGameState)))
    (Class|RPGSpawnManager|SpawnNewWave (Variables|/Script/RPG.RPG_GameStateBase|GetSpawnManager _asrpg_game_state_base))
    (CallFunction|RPGShowMessage (Game|GetPlayerController 0) "Monsters Spawned!" 5.0)
    (Audio|PlaySoundatLocation "/Game/Assets/Sounds/gong.gong" (Transformation|GetActorLocation) "0, 0, 0" 1.0 1.0 0.0 0 0 0)
    (bind _newtrack_0 (Timeline|Timeline_0 PlayFromStart)
      (:Update
        (Transformation|SetRelativeLocation (Variables|Default|GetSphere) (Math|Vector|MakeVector (+ (* _newtrack_0 1e+01) (.x _initpos)) (.y _initpos) (.z _initpos)) false false)))
    (else
      (CallFunction|RPGShowMessage (Game|GetPlayerController 0) "Eliminate all hostiles before spawning new wave!" 5.0))))

(fn ConstructionScript)

(fn GetInteractableType
  (return "MISC"))

(fn IsInteractable
  (return true))