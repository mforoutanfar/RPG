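; Interactable chest Blueprint that opens with a sound when interacted with and is written to support lockpicking.
; OnInteracted branches on the interactable type: a chest opens, while a locked chest either unlocks and opens on success or shows a locked message with a sound.
; GetInteractableType returns the plain chest type whether or not Locked is set, so the locked branch is never reached as written.
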(event EventBeginPlay)

(event Collision|EventActorBeginOverlap
  (params (OtherActor :type Actor%20Object%20Reference)))

(event EventTick
  (params (DeltaSeconds :type Float%20%28single-precision%29)))

(event EventOnInteracted
  (params (Successful :type Boolean))
  (bind _self self)
  (bind _returnvalue (CallFunction|GetInteractableType))
  (switch Utilities|FlowControl|Switch|SwitchonInteractableCategory _returnvalue
    (:CHEST
      (Class|RPGContainer|Open :!label _label)
      (Audio|PlaySound2D "/Game/Assets/Sounds/door_open0.door_open0" 1.0 1.0 0.0 0 0))
    (:LOCKED_CHEST
      (if Successful
        (Variables|Default|SetLocked false)
        (CallFunction|RPGShowMessage _self "Lock Picked!" 5.0)
        (goto _label)
        (else
          (CallFunction|RPGShowMessage _self "Locked" 3.0)
          (Audio|PlaySoundatLocation "/Game/Assets/Sounds/locked0.locked0" (Transformation|GetActorLocation) "0, 0, 0" 1.0 1.0 0.0 0 0 0))))))

(fn ConstructionScript)

(fn GetInteractableType
  (if (Variables|Default|GetLocked)
    (return "LOCKED_CHEST")
    (else
      (return "CHEST"))))

(fn IsInteractable
  (return true))